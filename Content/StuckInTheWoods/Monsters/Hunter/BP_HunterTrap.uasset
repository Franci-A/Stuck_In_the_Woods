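; Hunter bear-trap-style hazard that snaps shut on a player character, damaging it and blocking its movement.
; It arms three seconds after spawning or being reopened, and a timeline rotates and moves the two jaw cubes.
; Repeated interactions fill a decaying meter that frees the victim and reopens the trap at a threshold.
; The trapped player's own interactions count at reduced strength, so other players open it faster.
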(event `self.ReceiveBeginPlay`
  (set `self.IsActive` false)
  (`self.TrapCooldown`))

(event `TrapAnimation`
  (params (CloseAnim :type Boolean))
  (bind _cube1 (`self.Cube1`))
  (bind _cube (`self.Cube`))
  (bind (_relativelocation_x _relativelocation_y) (`KismetMathLibrary.BreakVector` (`SceneComponent.RelativeLocation` _cube)))
  (bind (_relativelocation_x_2 _relativelocation_y_2) (`KismetMathLibrary.BreakVector` (`SceneComponent.RelativeLocation` _cube1)))
  (if CloseAnim
    (bind (_direction _position _rotation) (`Timeline|TrapAnim` :!via `PlayFromStart` :!label _label)
      (:`Update`
        (`SceneComponent.K2_SetRelativeRotation` (`self.Cube1`) (`KismetMathLibrary.MakeRotator` (* _rotation -1.0)) false false)
        (`SceneComponent.K2_SetRelativeRotation` (`self.Cube`) (`KismetMathLibrary.MakeRotator` _rotation) false false)
        (`SceneComponent.K2_SetRelativeLocation` _cube1 (`KismetMathLibrary.MakeVector` _relativelocation_x_2 _relativelocation_y_2 _position) false false)
        (`SceneComponent.K2_SetRelativeLocation` _cube (`KismetMathLibrary.MakeVector` _relativelocation_x _relativelocation_y _position) false false)))
    (else
      (goto _label :!via `ReverseFromEnd`))))

(event `TrapCooldown`
  (`KismetSystemLibrary.K2_SetTimerDelegate` (delegate `SetTrapActive`) 3.0))

(event `SetTrapActive`
  (set `self.IsActive` true))

(event `self.ReceiveActorBeginOverlap`
  (params (OtherActor :type "Actor Object Reference"))
  (if (and (not (`KismetSystemLibrary.IsValid` (`self.PlayerInTrap`))) (`self.IsActive`))
    (bind _asbp_main_character (cast `/Game/StuckInTheWoods/BP_MainCharacter` OtherActor))
    (set `self.IsActive` false)
    (bind _output_get (set `self.PlayerInTrap` _asbp_main_character))
    (`/Game/StuckInTheWoods/BP_MainCharacter.BlockPlayerMovement` _output_get true)
    (`/Game/StuckInTheWoods/Health_n_Damage/AC_Health.TakeDamage` (`/Game/StuckInTheWoods/BP_MainCharacter.AC_Health` _asbp_main_character) (`self.DamageAmount`))
    (`self.TrapAnimation` true)))

(event `/Game/StuckInTheWoods/Player/I_Interactable.OnInteract`
  (params (InteractingPlayer :type "/Game/StuckInTheWoods/BP_MainCharacter Object Reference"))
  (if (== (`self.PlayerInTrap`) InteractingPlayer)
    (set `self.CurrentAmount` (+ (* (`self.OpenAmountPerClick`) 0.7) (`self.CurrentAmount`)))
    (else
      (set `self.CurrentAmount` (+ (`self.OpenAmountPerClick`) (`self.CurrentAmount`)))))
  (if (>= (`self.CurrentAmount`) (`self.SpamAmountNeeded`))
    (`self.FreePlayer`)
    (set `self.CurrentAmount` 0.0)
    (`self.TrapCooldown`)
    (`self.TrapAnimation` false)))

(event `FreePlayer`
  (bind _playerintrap (`self.PlayerInTrap`))
  (if (`KismetSystemLibrary.IsValid` _playerintrap)
    (`/Game/StuckInTheWoods/BP_MainCharacter.BlockPlayerMovement` _playerintrap false)
    (set `self.PlayerInTrap` null)))

(event `self.ReceiveTick`
  (params (DeltaSeconds :type "Float (single-precision)"))
  (if (> (`self.CurrentAmount`) 0.0)
    (set `self.CurrentAmount` (- (`self.CurrentAmount`) (* DeltaSeconds 1.0)))))

(fn `UserConstructionScript`)