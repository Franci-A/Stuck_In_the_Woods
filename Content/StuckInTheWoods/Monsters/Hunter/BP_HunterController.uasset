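; AI controller for the Hunter monster that patrols and chases players within a territory centred on where it was possessed.
; On possess it runs BT_Hunter, writes territory center and radii to the blackboard, and starts a looping timer that re-enables trap placement.
; Perception sets the player as enemy, with a delayed timer clearing it on lost sight; Tick drops targets leaving the chase radius.
; Heard noises feed the blackboard as patrol locations.
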(event `self.ReceivePossess`
  (params (PossessedPawn :type "Pawn Object Reference"))
  (bind _returnvalue (`self.K2_GetActorLocation` PossessedPawn))
  (bind _blackboard (`self.Blackboard`))
  (bind _patrolradius (`self.PatrolRadius`))
  (bind _chaseradius (`self.ChaseRadius`))
  (`self.RunBehaviorTree` "/Game/StuckInTheWoods/Monsters/Hunter/BT_Hunter.BT_Hunter")
  (set `self.TerritoryCenterPoint` _returnvalue)
  (`BlackboardComponent.SetValueAsVector` _blackboard (`self.TerritoryCenter`) _returnvalue)
  (`BlackboardComponent.SetValueAsFloat` _blackboard (`self.PatrolRadiusKey`) _patrolradius)
  (`KismetSystemLibrary.DrawDebugSphere` _returnvalue _patrolradius 16 (struct :`R` 0.40223 :`G` 0.043877 :`B` 1.0 :`A` 1.0) 10.0 1.0)
  (`BlackboardComponent.SetValueAsFloat` _blackboard (`self.ChaseRadiusKey`) _chaseradius)
  (`KismetSystemLibrary.DrawDebugSphere` _returnvalue _chaseradius 16 (struct :`G` 0.25 :`B` 1.0 :`A` 1.0) 10.0 1.0)
  (`KismetSystemLibrary.K2_SetTimerDelegate` (delegate `SpawnTrapTimer`) 10.0 true))

(event `SpawnTrapTimer`
  (`BlackboardComponent.SetValueAsBool` (`self.Blackboard`) (`self.CanPlaceTrap`) true))

(event `self.ReceiveTick`
  (params (DeltaSeconds :type "Float (single-precision)"))
  (bind _targetactor (`self.TargetActor`))
  (if (`KismetSystemLibrary.IsValid` _targetactor)
    (if (> (`KismetMathLibrary.Vector_Distance` (`self.K2_GetActorLocation` _targetactor) (`self.TerritoryCenterPoint`)) (`self.ChaseRadius`))
      (`self.StartEnemyTimer`)
      (set `self.TargetActor` null)
      (`KismetSystemLibrary.PrintString` "outside range"))))

(event `self.AIPerception.OnTargetPerceptionUpdated`
  (params (Actor :type "Actor Object Reference") (Stimulus :type "AIStimulus Structure"))
  (bind _blackboard (`self.Blackboard`))
  (if (and (`self.ActorHasTag` Actor "Player") (`.bSuccessfullySensed` (break `AIStimulus` Stimulus)) (<= (`KismetMathLibrary.Vector_Distance` (`self.K2_GetActorLocation` Actor) (`self.TerritoryCenterPoint`)) (`self.ChaseRadius`)))
    (set `self.TargetActor` Actor)
    (`KismetSystemLibrary.PrintString` "see true")
    (`KismetSystemLibrary.K2_ClearAndInvalidateTimerHandle` (`self.EnemyTimer`))
    (`BlackboardComponent.SetValueAsBool` _blackboard (`self.HasLineOfSight`) true)
    (`BlackboardComponent.SetValueAsObject` _blackboard (`self.EnemyActor`) Actor)
    (else
      (bind _returnvalue (`KismetSystemLibrary.K2_SetTimerDelegate` (delegate `StartEnemyTimer`) (`self.LineOfSightTimer`)))
      (set `self.EnemyTimer` _returnvalue))))

(event `StartEnemyTimer`
  (bind _blackboard (`self.Blackboard`))
  (`BlackboardComponent.SetValueAsBool` _blackboard (`self.HasLineOfSight`) false)
  (`BlackboardComponent.SetValueAsObject` _blackboard (`self.EnemyActor`) null))

(event `self.BP_NoiseReceiver.OnNoiseReceived`
  (params (Location :type "Vector Structure") (Loudness :type "Float (double-precision)") (Tag :type String))
  (bind _blackboard (`self.Blackboard`))
  (`BlackboardComponent.SetValueAsBool` _blackboard (`self.HeardNoiseKey`) true)
  (`BlackboardComponent.SetValueAsVector` _blackboard (`self.PatrolLocationKey`) Location))

(event `StopNoiseSearch`
  (`BlackboardComponent.SetValueAsBool` (`self.Blackboard`) (`self.HeardNoiseKey`) false))

(fn `UserConstructionScript`)