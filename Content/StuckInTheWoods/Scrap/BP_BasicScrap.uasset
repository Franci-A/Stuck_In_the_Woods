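; BP_BasicScrap is a basic scrap object that yields randomized resource drops.
; On BeginPlay it runs the parent logic and assigns its Sphere as the visual reference, and GetParent returns the object itself.
; GetResources walks the ResourceValues map, rolls a random amount within each resource type's min/max range, and returns the resulting Drops list.
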(event `self.ReceiveBeginPlay`
  (`parent.ReceiveBeginPlay`)
  (set `self.VisualRef` (`self.Sphere`)))

(fn `GetParent`
  (returns (Parent :type "Actor Object Reference"))
  (return self))

(fn `GetResources`
  (returns (Resources :type "Set of /Game/StuckInTheWoods/Crafting_Receipes/Resource Structure"))
  (locals (Drops :type "Set of /Game/StuckInTheWoods/Crafting_Receipes/Resource Structure"))
  (bind _resourcevalues (`self.ResourceValues`))
  (bind _keys (`BlueprintMapLibrary.Map_Keys` _resourcevalues))
  (for _array_element _keys
    (bind (_min _max) (break `/Game/StuckInTheWoods/MinMax` (`BlueprintMapLibrary.Map_Find` _resourcevalues _array_element)))
    (`BlueprintSetLibrary.Set_Add` (`local.Drops`) (make `/Game/StuckInTheWoods/Crafting_Receipes/Resource` _array_element (`KismetMathLibrary.RandomIntegerInRange` _min _max))))
  (return (`local.Drops`)))

(fn `UserConstructionScript`)