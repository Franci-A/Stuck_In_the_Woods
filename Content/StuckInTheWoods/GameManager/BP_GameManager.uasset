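; Multiplayer game manager for StuckInTheWoods that spawns players, tracks their readiness and runs the door-gated night cycle.
; Login spawns and possesses a BP_MainCharacter at the first PlayerStart; logout uses a stored controller-to-player map to clean both player lists.
; Once all players toggle ready, BP_Door opens for a short timed cycle, then closes and readiness resets.
; It also pushes PlayerState nicknames and list changes to characters and the door widget.
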(event `self.ReceiveBeginPlay`
  ; Begin play
  (`|ExecutionSequence`
    (:`then_0`
      (bind _outactors (`GameplayStatics.GetAllActorsOfClass` "/Script/Engine.PlayerStart"))
      (set `self.PlayerStarts` _outactors)
      (`self.SpawnPlayer` (`GameplayStatics.GetPlayerControllerFromID` 0)))
    (:`then_1`
      (bind _returnvalue (`GameplayStatics.GetActorOfClass` "/Game/StuckInTheWoods/Cabin/BP_Door.BP_Door_C"))
      (if (`KismetSystemLibrary.IsValid` _returnvalue)
        (set `self.Door` _returnvalue)
        (set `/Game/StuckInTheWoods/Cabin/BP_Door.GameManager` self _returnvalue)))))

(event `RemovePlayer`
  (params (ControllerToRemove :type "Controller Object Reference") (Player :type "/Game/StuckInTheWoods/BP_MainCharacter Object Reference"))
  ; Store controller and player when a pawn is destroyed
  (`BlueprintMapLibrary.Map_Add` (`self.ControllerToRemove`) ControllerToRemove Player))

(event `self.K2_PostLogin`
  (params (NewPlayer :type "PlayerController Object Reference"))
  ; Event when logging in + when a player finish initialized
  (`self.SpawnPlayer` NewPlayer)
  (set `self.NumberOfPlayers` (`GameplayStatics.GetNumPlayerControllers`)))

(event `self.K2_OnLogout`
  (params (ExitingController :type "Controller Object Reference"))
  (bind (_value _returnvalue) (`BlueprintMapLibrary.Map_Find` (`self.ControllerToRemove`) ExitingController))
  ; When a player LogOut from the server
  (if _returnvalue
    ;; Remove the player from the player list
    (for _array_element (`self.Players`)
      (if (== _array_element _value)
        (`KismetArrayLibrary.Array_RemoveItem` (`self.Players`) _array_element)
        (break)))
    ;; Remove the player from the PlayerReadyList if he was ready to go
    (for _array_element_2 (`self.PlayerReady`)
      (if (== _array_element_2 _value)
        (`KismetArrayLibrary.Array_RemoveItem` (`self.PlayerReady`) _array_element_2)
        (break)))
    ;; Remove the player from ControllerToRemoved and check the door (to update the UI and start the cycle if needed)
    (`BlueprintMapLibrary.Map_Remove` (`self.ControllerToRemove`) ExitingController)
    (set `self.NumberOfPlayers` (- (`self.NumberOfPlayers`) 1))
    (`self.CheckDoor`)))

(event `PlayerJustInit`
  (params (NewParam :type "Controller Object Reference"))
  ; Event when logging in + when a player finish initialized
  (`KismetSystemLibrary.Delay` 2.0)
  (for _array_element (`self.Players`)
    (bind _asps_player_state (cast `/Game/StuckInTheWoods/PS_PlayerState` (`Controller.PlayerState` (`Pawn.GetController` _array_element)) :!label _label)
      (:`then`
        (`/Game/StuckInTheWoods/BP_MainCharacter.SetNicknameAll` _array_element (`/Game/StuckInTheWoods/PS_PlayerState.PlayerName` _asps_player_state))
        (`/Game/StuckInTheWoods/Cabin/BP_Door.UpdateWidget` (`self.Door`) (`self.Players`) (`self.PlayerReady`)))
      (:`CastFailed`
        (`KismetSystemLibrary.Delay` 0.1)
        (goto _label)))))

(event `CheckDoor`
  ; Ready up
  (if (>= (`KismetArrayLibrary.Array_Length` (`self.PlayerReady`)) (`self.NumberOfPlayers`)) :!label _label_2
    (`self.StartCycle`))
  (`/Game/StuckInTheWoods/Cabin/BP_Door.UpdateWidget` (`self.Door`) (`self.Players`) (`self.PlayerReady`) :!label _label_3))

(event `PlayerReadyUp`
  (params (Player :type "/Game/StuckInTheWoods/BP_MainCharacter Object Reference"))
  ; Ready up
  (if (`|EnumEquality` (`self.GameTimeState`) "NewEnumerator0")
    (if (== (`KismetArrayLibrary.Array_Find` (`self.PlayerReady`) Player) -1)
      (`KismetArrayLibrary.Array_Add` (`self.PlayerReady`) Player)
      (goto _label_2)
      (else
        (`KismetArrayLibrary.Array_RemoveItem` (`self.PlayerReady`) Player)
        (goto _label_3)))))

(event `StartCycle`
  ; Start Night cycle
  (`KismetSystemLibrary.K2_SetTimerDelegate` (delegate `EndCycle`) 10.0)
  (`KismetSystemLibrary.PrintString` "start cycle" true true (struct :`G` 0.66 :`B` 1.0 :`A` 1.0) 5.0)
  (set `self.GameTimeState` "NewEnumerator1")
  (`/Game/StuckInTheWoods/Cabin/BP_Door.OpenDoor` (`self.Door`)))

(event `EndCycle`
  ; End Night cycle
  (`KismetSystemLibrary.PrintString` "end cycle" true true (struct :`G` 0.66 :`B` 1.0 :`A` 1.0) 5.0)
  (`KismetArrayLibrary.Array_Clear` (`self.PlayerReady`))
  (set `self.GameTimeState` "NewEnumerator0")
  (`/Game/StuckInTheWoods/Cabin/BP_Door.CloseDooor` (`self.Door`))
  (`/Game/StuckInTheWoods/Cabin/BP_Door.UpdateWidget` (`self.Door`) (`self.Players`) (`self.PlayerReady`)))

(fn `SpawnPlayer`
  (params (PlayerController :type "PlayerController Object Reference"))
  (bind _returnvalue (`Controller.K2_GetPawn` PlayerController))
  (`/Engine/EditorBlueprintResources/StandardMacros.IsValid` _returnvalue
    (:`Is Valid`
      (bind _asbp_main_character (cast `/Game/StuckInTheWoods/BP_MainCharacter` _returnvalue)
        (:`then`
          (`KismetArrayLibrary.Array_RemoveItem` (`self.Players`) _asbp_main_character)
          (`self.K2_DestroyActor` _returnvalue))
        (:`CastFailed`
          _)))
    (:`Is Not Valid`
      _))
  (bind _returnvalue_2 (`|SpawnActorFromClass` "/Game/StuckInTheWoods/BP_MainCharacter.BP_MainCharacter_C" (`KismetMathLibrary.Conv_VectorToTransform` (`self.K2_GetActorLocation` (`|GetArrayItem` (`self.PlayerStarts`)))) "Undefined" "MultiplyWithRoot" null null))
  (`KismetArrayLibrary.Array_Add` (`self.Players`) _returnvalue_2)
  (`Controller.Possess` PlayerController _returnvalue_2))

(fn `UserConstructionScript`)