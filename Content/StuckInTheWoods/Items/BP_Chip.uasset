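; BP_Chip is a held item that registers the player carrying it as chipped when used.
; BeginPlay runs the parent logic and sets the Cube component as the item's visual reference.
; Interact, only while in hand, passes the owning BP_MainCharacter to AddChippedPlayer on the BP_GameManager game mode.
; If that call returns true, the character is told the object was used and destroyed.
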(event `self.ReceiveBeginPlay`
  (`parent.ReceiveBeginPlay`)
  (set `self.VisualRef` (`self.Cube`)))

(event `/Game/StuckInTheWoods/Player/I_Pickupable.Interact`
  (if (`self.IsInHand`)
    (bind _asbp_game_manager (cast `/Game/StuckInTheWoods/GameManager/BP_GameManager` (`GameplayStatics.GetGameMode`)))
    (bind _asbp_main_character (cast `/Game/StuckInTheWoods/BP_MainCharacter` (`self.GetOwner`)))
    (bind _isadded (`/Game/StuckInTheWoods/GameManager/BP_GameManager.AddChippedPlayer` _asbp_game_manager _asbp_main_character))
    (if _isadded
      (`/Game/StuckInTheWoods/BP_MainCharacter.ObjectUsedAndDestroyed` _asbp_main_character true))))

(fn `UserConstructionScript`
  (`parent.UserConstructionScript`))