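; BP_BaseItemRechargeable is a base item Blueprint for items with a battery that can be recharged.
; It fills CurrentBattery to MaxBattery on BeginPlay.
; The Recharge event adds the supplied energy as a fraction of MaxBattery, with no clamp to the maximum.
; NeededToRecharge is a stub that always returns zero.
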(event `self.ReceiveBeginPlay`
  ; Set CurrentBattery to MaxBattery
  (`parent.ReceiveBeginPlay`)
  (set `self.CurrentBattery` (`self.MaxBattery`)))

(event `/Game/StuckInTheWoods/Player/I_Pickupable.Recharge`
  (params (EnergyGet :type "Float (double-precision)"))
  ; Recharge
  (set `self.CurrentBattery` (+ (`self.CurrentBattery`) (* EnergyGet (`self.MaxBattery`)))))

(fn `NeededToRecharge`
  (returns (TrueEnergyNeeded :type "Float (double-precision)"))
  (return 0.0))

(fn `UserConstructionScript`
  (`parent.UserConstructionScript`))