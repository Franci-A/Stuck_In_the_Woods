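; Base item actor that players can pick up, hold, hide and drop.
; Interaction hands the item to the player's OnPickup if inventory slots are free; Pickup disables collision, attaches to the "Item slot" socket and records the owning Pawn.
; Show/hide toggles mesh visibility and the in-hand flag, adding or removing the item's widget only for the local controller.
; Drop removes that widget, restores collision, detaches at the given position and clears ownership.
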(event `/Game/StuckInTheWoods/Player/I_Interactable.OnInteract`
  (params (InteractingPlayer :type "/Game/StuckInTheWoods/BP_MainCharacter Object Reference"))
  ;[1 1 1 0.5] Interact + Pickup
  (bind _hasslot (`/Game/StuckInTheWoods/BP_MainCharacter.HasInventorySlots` InteractingPlayer))
  (if _hasslot
    (`/Game/StuckInTheWoods/BP_MainCharacter.OnPickup` InteractingPlayer self)))

(event `/Game/StuckInTheWoods/Player/I_Pickupable.Pickup`
  (params (ParentActor :type "Actor Object Reference") (Location :type "Vector Structure") (Pawn :type "Controller Object Reference"))
  ;[1 1 1 0.5] Interact + Pickup
  (`PrimitiveComponent.SetCollisionEnabled` (`self.VisualRef`) "NoCollision")
  (`self.K2_AttachToActor` self ParentActor "Item slot" "SnapToTarget" "SnapToTarget" "SnapToTarget" false)
  (`self.K2_SetActorLocation` self Location false true)
  (set `self.ParentController` Pawn)
  (`self.SetOwner` Pawn))

(event `/Game/StuckInTheWoods/Player/I_Pickupable.ShowHideItem`
  (params (HideItem :type Boolean))
  (bind _parentcontroller (`self.ParentController`))
  ;[1 1 1 0.5] Show or Hide Item
  (set `self.IsInHand` (not HideItem))
  (`SceneComponent.SetHiddenInGame` (`self.VisualRef`) HideItem true)
  (`/Engine/EditorBlueprintResources/StandardMacros.IsValid` _parentcontroller
    (:`Is Valid`
      (if (`Controller.IsLocalController` _parentcontroller)
        (if HideItem
          (`Widget.RemoveFromParent` (`self.Widget`))
          (else
            (`UserWidget.AddToViewport` (`self.Widget`) 0)))))))

(event `/Game/StuckInTheWoods/Player/I_Pickupable.Drop`
  (params (Position :type "Vector Structure"))
  (bind _parentcontroller (`self.ParentController`))
  ;[1 1 1 0.5] Drop
  (`/Engine/EditorBlueprintResources/StandardMacros.IsValid` _parentcontroller
    (:`Is Valid`
      (if (`Controller.IsLocalController` _parentcontroller)
        (`Widget.RemoveFromParent` (`self.Widget`))))
    (:`Is Not Valid`
      _))
  (`PrimitiveComponent.SetCollisionEnabled` (`self.VisualRef`) "QueryAndPhysics")
  (`self.K2_DetachFromActor` self "KeepRelative" "KeepRelative" "KeepRelative")
  (`self.K2_SetActorLocation` self Position false true)
  (set `self.ParentController` null)
  (`self.SetOwner` null))

(fn `GetParent`
  (returns (Parent :type "Actor Object Reference"))
  (return null))

(fn `UserConstructionScript`)