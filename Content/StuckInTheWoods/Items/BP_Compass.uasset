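; BP_Compass is a pickup item whose needle holds a set world direction.
; Interacting hands it to the player if inventory slots are free, and pickup disables collision and attaches it to the new parent.
; A looping timer re-orients the needle root from PointDirection and world up, keeping it level as the compass moves.
; The timer starts on pickup or show and stops when the item is hidden, avoiding per-frame Tick updates.
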(event `/Game/StuckInTheWoods/Player/I_Interactable.OnInteract`
  (params (InteractingPlayer :type "/Game/StuckInTheWoods/BP_MainCharacter Object Reference"))
  (bind _hasslot (`/Game/StuckInTheWoods/BP_MainCharacter.HasInventorySlots` InteractingPlayer))
  (if _hasslot
    (`/Game/StuckInTheWoods/BP_MainCharacter.OnPickup` InteractingPlayer self)))

(event `/Game/StuckInTheWoods/Player/I_Pickupable.Pickup`
  (params (ParentActor :type "Actor Object Reference") (Location :type "Vector Structure") (Pawn :type "Controller Object Reference"))
  (bind _output_get (set `self.ParentActor` ParentActor))
  (`PrimitiveComponent.SetCollisionEnabled` (`self.Cylinder`) "NoCollision")
  (`self.K2_AttachToActor` _output_get "None" "SnapToTarget" "SnapToTarget" "SnapToTarget" false)
  (`self.K2_SetActorLocation` Location false true)
  (`self.StartNeedleDirectionTimer`))

(event `/Game/StuckInTheWoods/Player/I_Pickupable.ShowHideItem`
  (params (HideItem :type Boolean))
  (`SceneComponent.SetHiddenInGame` (`self.Cylinder`) HideItem true)
  (if HideItem
    (`self.StopNeedleDirectionTimer`)
    (else
      (`self.StartNeedleDirectionTimer`))))

(event `StartNeedleDirectionTimer`
  (bind _returnvalue (`KismetSystemLibrary.K2_SetTimerDelegate` (delegate `SetNeedleDirection`) (`self.NeedleUpdateTimer`) true))
  (set `self.SetNeedleDirectionTimer` _returnvalue))

(event `StopNeedleDirectionTimer`
  (bind _setneedledirectiontimer (`self.SetNeedleDirectionTimer`))
  (if (`KismetSystemLibrary.K2_IsValidTimerHandle` _setneedledirectiontimer)
    (`KismetSystemLibrary.K2_ClearAndInvalidateTimerHandle` _setneedledirectiontimer)))

(event `SetNeedleDirection`
  (`SceneComponent.K2_SetWorldRotation` (`self.NeedleRoot`) (`KismetMathLibrary.MakeRotFromYZ` (`self.PointDirection`) (`KismetMathLibrary.Vector_Up`)) false false))

(fn `GetParent`
  (returns (Parent :type "Actor Object Reference"))
  (return null))

(fn `UserConstructionScript`)