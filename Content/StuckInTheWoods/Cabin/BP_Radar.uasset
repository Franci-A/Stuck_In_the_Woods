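; BP_Radar is a cabin monitor whose scene capture camera follows a chipped player.
; Each tick, the capture component moves to the target's location plus an offset.
; Shortly after BeginPlay and on each interaction, authority calls InteractServer, then InteractAll, which asks BP_GameManager (the game mode) for the next chipped player by ID.
; If none is valid, the radar targets itself.
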(event `self.ReceiveTick`
  (params (DeltaSeconds :type "Float (single-precision)"))
  ; If there is a target, the camera follow the target with an offset
  (`/Engine/EditorBlueprintResources/StandardMacros.IsValid` (`self.TargetToFollow`)
    (:`Is Valid`
      (`SceneComponent.K2_SetWorldLocation` (`self.SceneCaptureComponent2D`) (+ (`self.K2_GetActorLocation` (`self.TargetToFollow`)) (`self.OffsetToFollow`)) false false))))

(event `self.ReceiveBeginPlay`
  ; Switch player to follow on the monitor + replication
  (`KismetSystemLibrary.Delay` 0.5)
  (`/Engine/EditorBlueprintResources/ActorMacros.Switch Has Authority` :!label _label
    (:`Authority`
      (`self.InteractServer`))))

(event `/Game/StuckInTheWoods/Player/I_Interactable.OnInteract`
  (params (InteractingPlayer :type "/Game/StuckInTheWoods/BP_MainCharacter Object Reference"))
  ; Switch player to follow on the monitor + replication
  (goto _label))

(event `InteractServer`
  ; Switch player to follow on the monitor + replication
  (`self.InteractAll`))

(event `InteractAll`
  ; Switch player to follow on the monitor + replication
  (bind _asbp_game_manager (cast `/Game/StuckInTheWoods/GameManager/BP_GameManager` (`GameplayStatics.GetGameMode`)))
  (bind (_player _newid) (`/Game/StuckInTheWoods/GameManager/BP_GameManager.GetPlayerWithID` _asbp_game_manager (+ (`self.CurrentID`) 1) true))
  (`/Engine/EditorBlueprintResources/StandardMacros.IsValid` _player
    (:`Is Valid`
      (set `self.TargetToFollow` _player)
      (set `self.CurrentID` _newid))
    (:`Is Not Valid`
      (set `self.TargetToFollow` self))))

(fn `UserConstructionScript`)