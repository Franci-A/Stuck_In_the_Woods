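; BP_CabinInventory is the cabin's resource inventory, tracking amounts per resource type in a Stock map.
; GetResourceAmount returns the stored amount, or zero when the type is absent.
; AddResource adds a resource's amount to any existing total and prints the change on screen.
; TakeResource subtracts the amount and writes it back without checking that enough is in stock.
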(fn `AddResource`
  (params (Resource :type "/Game/StuckInTheWoods/Crafting_Receipes/Resource Structure"))
  (bind (_type _amount) (break `/Game/StuckInTheWoods/Crafting_Receipes/Resource` Resource))
  (bind _stock (`self.Stock`))
  (bind (_value _returnvalue) (`BlueprintMapLibrary.Map_Find` _stock _type))
  (bind _returnvalue_2 (`KismetMathLibrary.SelectInt` (+ _value _amount) _amount _returnvalue))
  (`BlueprintMapLibrary.Map_Add` _stock _type _returnvalue_2) ; Adding new amount + existing value if found
  (`KismetSystemLibrary.PrintString` null (`KismetStringLibrary.Concat_StrStr` "Added " (`KismetStringLibrary.Conv_IntToString` _amount) "" (`|GetEnumeratorNameAsString` _type) " (" (`KismetStringLibrary.Conv_IntToString` _returnvalue_2) ")")))

(fn `GetResourceAmount`
  (params (Resource :type "/Game/StuckInTheWoods/Crafting_Receipes/E_ResourceType Enum" :default "NewEnumerator0"))
  (returns (Amount :type Integer))
  (bind (_value _returnvalue) (`BlueprintMapLibrary.Map_Find` (`self.Stock`) Resource))
  (return (`KismetMathLibrary.SelectInt` _value 0 _returnvalue)))

(fn `TakeResource`
  (params (Resource :type "/Game/StuckInTheWoods/Crafting_Receipes/Resource Structure (by ref)"))
  (bind (_type _amount) (break `/Game/StuckInTheWoods/Crafting_Receipes/Resource` Resource))
  (bind _stock (`self.Stock`))
  (`BlueprintMapLibrary.Map_Add` _stock _type (- (`BlueprintMapLibrary.Map_Find` _stock _type) _amount)))