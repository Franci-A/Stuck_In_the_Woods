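; BP_BatteryManager is an interactable power store that takes in batteries and recharges the player's held items.
; On interact, a held Item_Battery is removed from the inventory and destroyed, adding its value to the charge unless already full.
; Items implementing I_Rechargeable receive the fraction of their needed energy the store can cover, which is then deducted.
; A widget component's WBP_BatteryManager progress bar shows the current charge ratio.
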(event `UpdateWidget`
  ; Update UI
  (`/Game/StuckInTheWoods/Cabin/WBP_BatteryManager.UpdateProgressBar` (`self.BatteryWidget`) (/ (`self.CurrentBattery`) (`self.MaxBattery`))))

(event `self.ReceiveBeginPlay`
  ; Set Widget and Update
  (bind _aswbp_battery_manager (cast `/Game/StuckInTheWoods/Cabin/WBP_BatteryManager` (`WidgetComponent.GetWidget` (`self.Widget`))))
  (set `self.BatteryWidget` _aswbp_battery_manager)
  (`self.UpdateWidget`))

(event `/Game/StuckInTheWoods/Player/I_Interactable.OnInteract`
  (params (InteractingPlayer :type "/Game/StuckInTheWoods/BP_MainCharacter Object Reference"))
  (bind _bp_inventory (`/Game/StuckInTheWoods/BP_MainCharacter.BP_Inventory` InteractingPlayer))
  ; When a player interact with the BatteryManager
  (bind _iteminhand (`/Game/StuckInTheWoods/Player/BP_Inventory.GetItemInHand` _bp_inventory))
  (if (`KismetSystemLibrary.IsValidInterface` _iteminhand)
    (bind _asitem_battery (cast `/Game/StuckInTheWoods/Items/Item_Battery` _iteminhand)
      (:`then`
        ;;[0.06703 0.15 0.09153 0.5] If the item in hand is a Battery and CurrentBattery is not full, refill the battery of the BatteryManager
        (if (not (== (`self.CurrentBattery`) (`self.MaxBattery`)))
          (`/Game/StuckInTheWoods/Player/BP_Inventory.RemoveItemFromInventory` _bp_inventory _iteminhand)
          (`self.K2_AttachToActor` _asitem_battery self "None" "KeepWorld" "KeepWorld" "KeepWorld" false)
          (set `self.CurrentBattery` (`KismetMathLibrary.FClamp` (+ (`self.CurrentBattery`) (`/Game/StuckInTheWoods/Items/Item_Battery.BatteryValue` _asitem_battery)) 0.0 (`self.MaxBattery`)))
          (`self.UpdateWidget`)
          (`self.K2_DestroyActor` _asitem_battery)))
      (:`CastFailed`
        (bind _asi_rechargeble (cast `/Game/StuckInTheWoods/Player/I_Rechargeable` _iteminhand))
        ;;[0.1233 0.1286 0.15 0.5] If an item is rechargeable, check the energy needed and recharge it
        (bind _trueenergyneeded (`/Game/StuckInTheWoods/Player/I_Rechargeable.NeededToRecharge` _asi_rechargeble))
        (bind _returnvalue (`KismetMathLibrary.FClamp` (/ (`self.CurrentBattery`) _trueenergyneeded)))
        (`/Game/StuckInTheWoods/Player/I_Rechargeable.Recharge` _asi_rechargeble _returnvalue)
        (set `self.CurrentBattery` (- (`self.CurrentBattery`) (* _trueenergyneeded _returnvalue)))
        (`self.UpdateWidget`)))))

(fn `UserConstructionScript`)