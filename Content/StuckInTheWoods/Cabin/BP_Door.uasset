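; BP_Door is an interactable cabin door that either registers player ready-up or swings open and closed.
; On interact, the authority checks the GameManager time state, readying the player in one specific state and toggling the door otherwise.
; A single timeline plays or reverses to offset the door's yaw from its starting value.
; An animation guard blocks overlapping requests, and the open flag flips when the timeline finishes.
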(event `self.ReceiveBeginPlay`
  (bind (_relativerotation_roll _relativerotation_pitch _relativerotation_yaw) (`KismetMathLibrary.BreakRotator` (`SceneComponent.RelativeRotation` (`self.Door`))))
  (set `self.BaseYaw` _relativerotation_yaw))

(event `/Game/StuckInTheWoods/Player/I_Interactable.OnInteract`
  (params (InteractingPlayer :type "/Game/StuckInTheWoods/BP_MainCharacter Object Reference"))
  (`/Engine/EditorBlueprintResources/ActorMacros.Switch Has Authority`
    (:`Authority`
      (if (`|EnumEquality` (`/Game/StuckInTheWoods/GameManager/BP_GameManager.GameTimeState` (`self.GameManager`)) "NewEnumerator0")
        (`/Game/StuckInTheWoods/GameManager/BP_GameManager.PlayerReadyUp` (`self.GameManager`) InteractingPlayer)
        (else
          (`self.ToggleDoor`))))))

(event `OpenDoor`
  (`self.DoorAnimation` true))

(event `CloseDooor`
  (`self.DoorAnimation` false))

(event `ToggleDoor`
  (`self.DoorAnimation` (not (`self.IsOpen`))))

(event `DoorAnimation`
  (params (OpenDoor :type Boolean))
  ; Open door
  (if (not (`self.IsAnimating`))
    (set `self.IsAnimating` true)
    (if OpenDoor
      (bind (_direction _newtrack_0) (`Timeline|OpenDoor Timeline` :!label _label)
        (:`Update`
          (`SceneComponent.K2_SetRelativeRotation` (`self.Door`) (`KismetMathLibrary.MakeRotator` 0.0 0.0 (- (`self.BaseYaw`) _newtrack_0)) false false))
        (:`Finished`
          (set `self.IsAnimating` false)
          (set `self.IsOpen` (not (`self.IsOpen`)))))
      (else
        (goto _label :!via `Reverse`)))))

(fn `UserConstructionScript`)