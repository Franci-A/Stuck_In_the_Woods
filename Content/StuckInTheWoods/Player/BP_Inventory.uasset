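; BP_Inventory is the player's fixed-size item inventory, tracking a current slot as the item in hand.
; New items fill the current slot if empty, otherwise the first free one, which becomes current.
; Cycling wraps around the slots and toggles item visibility through an interface, so only the held item shows.
; Adding, removing and switching items notify the inventory widget.
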(event `self.ReceiveBeginPlay`
  ; Begin play
  (for _ (range (`self.InventorySize`))
    (`KismetArrayLibrary.Array_Add` (`self.Inventory slots`))))

(event `NextSlotIndex`
  (params (Add :type Integer))
  (bind _inventorywidget (`self.InventoryWidget`))
  (bind _returnvalue (+ (`self.CurrentIndex`) Add))
  ; Switch item in hand
  (if (>= _returnvalue (`self.InventorySize`))
    (set `self.CurrentIndex` 0)
    (elif (< _returnvalue 0)
      (set `self.CurrentIndex` (- (`self.InventorySize`) 1))
      (else
        (set `self.CurrentIndex` _returnvalue))))
  (`self.ShowItemInHand`)
  (`/Engine/EditorBlueprintResources/StandardMacros.IsValid` _inventorywidget
    (:`Is Valid`
      (`/Game/StuckInTheWoods/Player/W_Inventory.Selected Item Updated` _inventorywidget (`self.CurrentIndex`)))))

(event `AddToInventory`
  (params (Item :type "/Game/StuckInTheWoods/Player/I_Pickupable Interface"))
  (bind _inventorywidget (`self.InventoryWidget`))
  ; Add item
  (bind _index (`self.GetFirstEmptySlot`))
  (bind _output_get (set `self.CurrentIndex` _index))
  (`KismetSystemLibrary.PrintString` (`KismetStringLibrary.Conv_IntToString` _output_get))
  (`KismetArrayLibrary.Array_Set` (`self.Inventory slots`) _index Item)
  (`self.ShowItemInHand`)
  (`/Engine/EditorBlueprintResources/StandardMacros.IsValid` _inventorywidget
    (:`Is Valid`
      (`/Game/StuckInTheWoods/Player/W_Inventory.Item Added To Inventory` _inventorywidget (`self.CurrentIndex`)))))

(event `ShowItemInHand`
  (for (_array_element _array_index) (`self.Inventory slots`)
    (if (`KismetSystemLibrary.IsValidInterface` _array_element)
      (`/Game/StuckInTheWoods/Player/I_Pickupable.ShowHideItem` _array_element (not (== _array_index (`self.CurrentIndex`)))))))

(fn `GetFirstEmptySlot`
  (returns (index :type Integer))
  (if (`KismetSystemLibrary.IsValidInterface` (`|GetArrayItem` (`self.Inventory slots`) (`self.CurrentIndex`)))
    (for (_array_element _array_index) (`self.Inventory slots`)
      (if (not (`KismetSystemLibrary.IsValidInterface` _array_element))
        (return _array_index)))
    (`KismetSystemLibrary.PrintString` "No empty slot in inventory")
    (return -1)
    (else
      (return (`self.CurrentIndex`)))))

(fn `GetItemInHand`
  (returns (ItemInHand :type "/Game/StuckInTheWoods/Player/I_Pickupable Interface"))
  (return (`|GetArrayItem` (`self.Inventory slots`) (`self.CurrentIndex`))))

(fn `HasInventorySpace`
  (returns (HasSlot :type Boolean))
  (bind _index (`self.GetFirstEmptySlot`))
  (return (not (== _index -1))))

(fn `RemoveItemFromInventory`
  (params (Item :type "/Game/StuckInTheWoods/Player/I_Pickupable Interface"))
  (locals (Index :type Integer :default 0))
  (bind _inventory_slots (`self.Inventory slots`))
  (bind _output_get (set `local.Index` (`KismetArrayLibrary.Array_Find` _inventory_slots Item)))
  (`KismetArrayLibrary.Array_Set` _inventory_slots _output_get)
  (`/Game/StuckInTheWoods/Player/W_Inventory.Remove Item From Inventory` (`self.InventoryWidget`) _output_get))