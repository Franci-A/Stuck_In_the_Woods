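; BP_NoiseEmitter is a component that lets its owning actor emit noises for AI hearing perception.
; On BeginPlay it finds the owner's perception stimuli source and activates it, registering it for hearing, or prints an error if none exists.
; While that source is active, MakeNoise reports a tagged noise event at the owner's location, calls OnNoiseEmitted and prints debug output, with an optional loudness-scaled circle.
; Debug events toggle the emitter and trigger single or looping random-loudness noises.
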(event `self.ReceiveBeginPlay`
  (bind _returnvalue (`Actor.GetComponentByClass` (`self.GetOwner`) "/Script/AIModule.AIPerceptionStimuliSourceComponent"))
  (`/Engine/EditorBlueprintResources/StandardMacros.IsValid` _returnvalue
    (:`Is Valid`
      (set `self.PerceptionStimuliComponent` _returnvalue)
      (`self.SetActiveEmitter` true))
    (:`Is Not Valid`
      (`KismetSystemLibrary.PrintString` (`KismetStringLibrary.Concat_StrStr` (`KismetSystemLibrary.GetObjectName` (`self.PerceptionStimuliComponent`)) " wasn't found on Actor" (`KismetSystemLibrary.GetDisplayName` (`self.GetOwner`))) true true (struct :`R` 1.0 :`A` 1.0) 10.0))))

(event `Debug_NoiseLoop`
  ; Debug Functions
  (set `self.Debug_IsNoiseLooping` true)
  (if (`self.Debug_IsNoiseLooping`) :!label _label
    (`self.MakeNoise` (`KismetMathLibrary.RandomFloatInRange` 0.0 1.0))
    (`KismetSystemLibrary.Delay` 0.66)
    (goto _label)))

(event `SetActiveEmitter`
  (params (Active :type Boolean))
  (bind _perceptionstimulicomponent (`self.PerceptionStimuliComponent`))
  (`self.SetActive` _perceptionstimulicomponent Active false)
  (if Active
    (`AIPerceptionStimuliSourceComponent.RegisterForSense` _perceptionstimulicomponent "/Script/AIModule.AISense_Hearing")
    (else
      (`AIPerceptionStimuliSourceComponent.UnregisterFromSense` _perceptionstimulicomponent "/Script/AIModule.AISense_Hearing"))))

(event `Debug_StopLoop`
  ; Debug Functions
  (set `self.Debug_IsNoiseLooping` false))

(event `Debug_MakeNoise`
  ; Debug Functions
  (`self.MakeNoise` (`self.Debug_NoiseLoudness`)))

(event `Debug_Activate`
  ; Debug Functions
  (`self.SetActiveEmitter` true))

(event `Debug_Deactivate`
  ; Debug Functions
  (`self.SetActiveEmitter` false))

(event `MakeNoise`
  (params (Loudness :type "Float (single-precision)"))
  (bind _perceptionstimulicomponent (`self.PerceptionStimuliComponent`))
  (bind _returnvalue (`self.GetOwner` _perceptionstimulicomponent))
  (bind _returnvalue_2 (`Actor.K2_GetActorLocation` _returnvalue))
  (if (`self.IsActive` _perceptionstimulicomponent)
    (`AISense_Hearing.ReportNoiseEvent` _returnvalue_2 Loudness _returnvalue 0.0 "NOISE_")
    (`self.OnNoiseEmitted` _returnvalue_2 Loudness "NOISE_")
    ; Debugging
    (`KismetSystemLibrary.PrintString` (`KismetStringLibrary.Concat_StrStr` "Making Noise from " (`KismetSystemLibrary.GetDisplayName` _returnvalue) ", at " (`KismetStringLibrary.Conv_VectorToString` _returnvalue_2) ". Volume: " (`KismetStringLibrary.Conv_DoubleToString` Loudness)) true true (struct :`R` 0.322917 :`G` 0.769792 :`B` 1.0 :`A` 1.0))
    (if (`self.DrawDebug`)
      (`KismetSystemLibrary.DrawDebugCircle` _returnvalue_2 120.0 12 (`KismetMathLibrary.LinearColorLerp` (struct :`R` 0.358854 :`G` 0.988 :`A` 1.0) (struct :`R` 1.0 :`G` 0.08 :`A` 1.0) Loudness) 0.0 (`KismetMathLibrary.Lerp` 0.2 1.5 Loudness) (0.0 1.0 0.0) (1.0 0.0 0.0) true))))