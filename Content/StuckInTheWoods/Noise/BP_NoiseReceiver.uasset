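; Noise receiver component that lets its owning actor hear tagged noises through a perception component and relay them as an event.
; On BeginPlay it binds to the owner's perception component and activates it, only printing a message if none exists.
; On authority, successfully sensed "NOISE"-tagged stimuli pass location, loudness and tag through a MULTI event to OnNoiseReceived.
; Optional debug drawing shows spheres around the owner and strength-scaled arrows toward heard noises.
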(event `self.ReceiveBeginPlay`
  (bind _returnvalue (`self.GetOwner`))
  (bind _returnvalue_2 (`Actor.GetComponentByClass` _returnvalue (`self.TargetComponentClass`)))
  (`/Engine/EditorBlueprintResources/StandardMacros.IsValid` _returnvalue_2
    (:`Is Valid`
      (`self.InitPerceptionComponent` _returnvalue_2))
    (:`Is Not Valid`
      (`KismetSystemLibrary.PrintString` (`KismetStringLibrary.Concat_StrStr` "PawnSensing Component" " wasn't found on Actor " (`KismetSystemLibrary.GetDisplayName` _returnvalue) ". -> Adding Component...") true true (struct :`R` 1.0 :`A` 1.0) 10.0))))

(event `InitPerceptionComponent`
  (params (PerceptionComponent :type "AIPerceptionComponent Object Reference"))
  (bind _output_get (set `self.PerceptionComponent` PerceptionComponent))
  (`self.SetActiveReceiver` true)
  (add `AIPerceptionComponent.OnTargetPerceptionUpdated` _output_get (delegate `OnTargetPerceptionUpdated`)))

(event `Debug_Activate`
  ; Debug Functions
  (`self.SetActiveReceiver` true))

(event `Debug_Deactivate`
  ; Debug Functions
  (`self.SetActiveReceiver` false))

(event `SetActiveReceiver`
  (params (Active :type Boolean))
  (`self.SetActive` (`self.PerceptionComponent`) Active false))

(event `OnTargetPerceptionUpdated`
  (params (Actor :type "Actor Object Reference") (Stimulus :type "AIStimulus Structure"))
  (bind (_age _expirationage _strength _stimuluslocation _receiverlocation _tag _bsuccessfullysensed) (break `AIStimulus` Stimulus))
  (bind _returnvalue (`KismetStringLibrary.Conv_NameToString` _tag))
  (`/Engine/EditorBlueprintResources/ActorComponentMacros.Switch Has Authority`
    (:`Authority`
      (if (and (`self.IsActive` (`self.PerceptionComponent`)) _bsuccessfullysensed (`KismetStringLibrary.Contains` _returnvalue "NOISE"))
        (`self.CallOnNoiseReceived_MULTI` _stimuluslocation _strength _returnvalue)
        ; Debugging
        (`KismetSystemLibrary.PrintString` (`KismetStringLibrary.Concat_StrStr` "Heard Noise from " (`KismetSystemLibrary.GetObjectName` Actor) ", at " (`KismetStringLibrary.Conv_VectorToString` _stimuluslocation) ". Strength: " (`KismetStringLibrary.Conv_DoubleToString` _strength)) true true (struct :`R` 0.10026 :`G` 0.639089 :`B` 0.916667 :`A` 1.0))
        (if (`self.DrawDebug`)
          (`KismetSystemLibrary.DrawDebugArrow` (`Actor.K2_GetActorLocation` (`self.GetOwner`)) _stimuluslocation 0.5 (`KismetMathLibrary.LinearColorLerp` (struct :`R` 0.358854 :`G` 0.988 :`A` 1.0) (struct :`R` 1.0 :`G` 0.08 :`A` 1.0) _strength) _expirationage (`KismetMathLibrary.Lerp` 0.2 1.5 _strength)))))))

(event `self.ReceiveTick`
  (params (DeltaSeconds :type "Float (single-precision)"))
  (bind _returnvalue (`Actor.K2_GetActorLocation` (`self.GetOwner`)))
  ; Debugging
  (if (`self.DrawDebug`)
    (`KismetSystemLibrary.DrawDebugSphere` _returnvalue 100.0 12 (struct :`G` 1.0 :`B` 0.243758 :`A` 1.0) 0.0 0.5)
    (`KismetSystemLibrary.DrawDebugSphere` _returnvalue 100.0 12 (struct :`R` 1.0 :`G` 0.719981 :`A` 1.0) 0.0 0.5)))

(event `CallOnNoiseReceived_MULTI`
  (params (Location :type "Vector Structure") (Loudness :type "Float (double-precision)") (Tag :type String))
  (`self.OnNoiseReceived` Location Loudness Tag))