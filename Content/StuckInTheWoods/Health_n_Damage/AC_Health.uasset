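; Health component that tracks an actor's current and maximum health and reports damage and death.
; Health starts at max on BeginPlay, and SetHealthValue clamps changes before broadcasting the update.
; TakeDamage lowers health through that setter, then subtracts Amount again in its check, so death can fire while health remains above zero.
; Changing max health broadcasts its own update without re-clamping current health.
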(event `self.ReceiveBeginPlay`
  (`self.InitHealthValue`))

(event `InitHealthValue`
  (set `self.CurrentHealthValue` (`self.MaxHealth`)))

(event `/Game/StuckInTheWoods/Health_n_Damage/IDamageable.TakeDamage`
  (params (Amount :type "Float (double-precision)"))
  (bind _returnvalue (- (`self.CurrentHealthValue`) Amount))
  (`self.SetHealthValue` _returnvalue)
  (if (> _returnvalue 0.0)
    (`self.OnDamageTaken` Amount)
    (else
      (`self.OnDeath`))))

(event `SetHealthValue`
  (params (Value :type "Float (double-precision)"))
  (bind _output_get (set `self.CurrentHealthValue` (`KismetMathLibrary.FClamp` Value 0.0 (`self.MaxHealth`))))
  (`self.OnHealthUpdate` _output_get))

(event `SetMaxHealthValue`
  (params (Value :type "Float (double-precision)"))
  (bind _output_get (set `self.MaxHealth` Value))
  (`self.OnMaxHealthUpdate` _output_get))