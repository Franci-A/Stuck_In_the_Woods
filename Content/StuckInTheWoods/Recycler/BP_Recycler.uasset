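; BP_Recycler is an interactable machine that turns a held BP_BasicScrap item into materials for the cabin.
; On interact, it takes the scrap from the player's inventory and attaches it above its cube mesh, with a flag blocking further input while busy.
; After a delay, it sends the scrap's wood, plastic, metal and electronic amounts to the referenced cabin, then destroys the item.
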(event `/Game/StuckInTheWoods/Player/I_Interactable.OnInteract`
  (params (InteractingPlayer :type "/Game/StuckInTheWoods/BP_MainCharacter Object Reference"))
  (bind _bp_inventory (`/Game/StuckInTheWoods/BP_MainCharacter.BP_Inventory` InteractingPlayer))
  (bind _iteminhand (`/Game/StuckInTheWoods/Player/BP_Inventory.GetItemInHand` _bp_inventory))
  (if (`KismetSystemLibrary.IsValidInterface` _iteminhand)
    (bind _parent (`/Game/StuckInTheWoods/Player/I_Pickupable.GetParent` _iteminhand))
    (bind _asbp_basic_scrap (cast `/Game/StuckInTheWoods/Scrap/BP_BasicScrap` _parent))
    (if (not (`self.IsRecycling`))
      (`/Game/StuckInTheWoods/Player/BP_Inventory.RemoveItemFromInventory` _bp_inventory _iteminhand)
      (set `self.IsRecycling` true)
      (`self.K2_AttachToActor` _asbp_basic_scrap self "None" "KeepWorld" "KeepWorld" "KeepWorld" false)
      (`self.K2_SetActorLocation` _asbp_basic_scrap (+ (`SceneComponent.K2_GetComponentLocation` (`self.Cube`)) (0.0 0.0 100.0)) false true)
      (`KismetSystemLibrary.Delay` (`self.RecycleTime`))
      (bind _scrapamount (`/Game/StuckInTheWoods/Scrap/BP_BasicScrap.GetAmountByType` _asbp_basic_scrap "NewEnumerator0"))
      (bind _scrapamount_2 (`/Game/StuckInTheWoods/Scrap/BP_BasicScrap.GetAmountByType` _asbp_basic_scrap "NewEnumerator1"))
      (bind _scrapamount_3 (`/Game/StuckInTheWoods/Scrap/BP_BasicScrap.GetAmountByType` _asbp_basic_scrap "NewEnumerator2"))
      (bind _scrapamount_4 (`/Game/StuckInTheWoods/Scrap/BP_BasicScrap.GetAmountByType` _asbp_basic_scrap "NewEnumerator3"))
      (`/Game/StuckInTheWoods/Cabin/BP_CabinManager.ReceiveScrap` (`self.CabinRef`) _scrapamount _scrapamount_2 _scrapamount_3 _scrapamount_4)
      (`self.K2_DestroyActor` _asbp_basic_scrap)
      (set `self.IsRecycling` false))))

(fn `UserConstructionScript`)